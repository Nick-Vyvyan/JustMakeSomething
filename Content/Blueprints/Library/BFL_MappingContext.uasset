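; Blueprint function library with shortcuts for adding and removing Enhanced Input mapping contexts on the first local player.
; Each function gets player controller 0 and its Enhanced Input local player subsystem, validity-checks both, then applies the given context.
; Contexts are always added at priority 0, and nothing happens if either check fails.
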(fn `EasyAddMappingContext`
  (params (`Mapping Context` :type "InputMappingContext Object Reference"))
  (bind _returnvalue (`GameplayStatics.GetPlayerController` null))
  (bind _returnvalue_2 (pcsubsystem `EnhancedInputLocalPlayerSubsystem` _returnvalue))
  (`/Engine/EditorBlueprintResources/StandardMacros.IsValid` _returnvalue
    (:`Is Valid`
      (`/Engine/EditorBlueprintResources/StandardMacros.IsValid` _returnvalue_2
        (:`Is Valid`
          (`EnhancedInputSubsystemInterface.AddMappingContext` _returnvalue_2 (`local.Mapping Context`) 0 (struct)))))))

(fn `EasyRemoveMappingContext`
  (params (`Mapping Context` :type "InputMappingContext Object Reference"))
  (bind _returnvalue (`GameplayStatics.GetPlayerController` null))
  (bind _returnvalue_2 (pcsubsystem `EnhancedInputLocalPlayerSubsystem` _returnvalue))
  (`/Engine/EditorBlueprintResources/StandardMacros.IsValid` _returnvalue
    (:`Is Valid`
      (`/Engine/EditorBlueprintResources/StandardMacros.IsValid` _returnvalue_2
        (:`Is Valid`
          (`EnhancedInputSubsystemInterface.RemoveMappingContext` _returnvalue_2 (`local.Mapping Context`) (struct)))))))