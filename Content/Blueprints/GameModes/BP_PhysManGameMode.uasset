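; BP_PhysManGameMode is a game mode that detects when every pickup item in the level has been picked up.
; On BeginPlay it caches all BP_PickupItem actors in an array.
; Each Tick, AllPickedUp scans that array's IsPickedUp flags, stopping at the first uncollected item.
; Once none remain, a DoOnce lets it print a single completion message.
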(event `self.ReceiveBeginPlay`
  (bind _outactors (`GameplayStatics.GetAllActorsOfClass` "/Game/Blueprints/Gameplay/BP_PickupItem.BP_PickupItem_C"))
  (set `self.PickUpItems` _outactors))

(event `self.ReceiveTick`
  (params (DeltaSeconds :type "Float (single-precision)"))
  (if (`self.AllPickedUp` (`self.PickUpItems`))
    (`/Engine/EditorBlueprintResources/StandardMacros.DoOnce` false
      (:`Completed`
        (`KismetSystemLibrary.PrintString` "ALL ITEMS PICKED UP")))))

(fn `AllPickedUp`
  (params (PickUpItems :type "Array of /Game/Blueprints/Gameplay/BP_PickupItem Object Reference"))
  (returns (AllPickedup :type Boolean))
  (locals (AnyNotPickedUp :type Boolean :default false) (NotPickedUp :type "Array of /Game/Blueprints/Gameplay/BP_PickupItem Object Reference"))
  (for _array_element PickUpItems
    (if (not (`/Game/Blueprints/Gameplay/BP_PickupItem.IsPickedUp` _array_element))
      (`KismetArrayLibrary.Array_Add` (`local.NotPickedUp`) _array_element)
      (break)))
  (return (`KismetArrayLibrary.Array_IsEmpty` (`local.NotPickedUp`))))

(fn `UserConstructionScript`)