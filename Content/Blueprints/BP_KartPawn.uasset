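; BP_KartPawn is the kart pawn, translating Enhanced Input actions into driving and camera control.
; BeginPlay adds the kart mapping context for player controller 0, then input events call helpers for acceleration, steering torque, camera look, handbrake and position reset.
; Releasing accelerate, steer or handbrake clears the matching state flag.
; The helper logic lies outside this event graph, and the construction script is empty.
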(event `self.ReceiveBeginPlay`
  (bind _returnvalue (pcsubsystem `EnhancedInputLocalPlayerSubsystem` (`GameplayStatics.GetPlayerController` 0)))
  (`/Engine/EditorBlueprintResources/StandardMacros.IsValid` _returnvalue
    (:`Is Valid`
      (`EnhancedInputSubsystemInterface.AddMappingContext` _returnvalue "/Game/Input/IMC_Kart.IMC_Kart" 0 (struct)))))

(event `EnhancedInput|/Game/Input/IA_Accelerate`
  (params (ActionValue :type "Float (double-precision)") (ElapsedSeconds :type "Float (double-precision)") (TriggeredSeconds :type "Float (double-precision)") (InputAction :type "InputAction Object Reference" :default "/Game/Input/IA_Accelerate.IA_Accelerate"))
  (:`Triggered`
    (`self.SetAccelerationInput` ActionValue))
  (:`Completed`
    (set `self.bHasAccelerationInput` false)))

(event `EnhancedInput|/Game/Input/IA_Steer`
  (params (ActionValue :type "Float (double-precision)") (ElapsedSeconds :type "Float (double-precision)") (TriggeredSeconds :type "Float (double-precision)") (InputAction :type "InputAction Object Reference" :default "/Game/Input/IA_Steer.IA_Steer"))
  (:`Triggered`
    (`self.ApplySteeringTorque` ActionValue))
  (:`Completed`
    (set `self.bHasSteeringInput` false)))

(event `EnhancedInput|/Game/Input/IA_CameraLook`
  (params (ActionValue :type "Vector2D Structure") (ElapsedSeconds :type "Float (double-precision)") (TriggeredSeconds :type "Float (double-precision)") (InputAction :type "InputAction Object Reference" :default "/Game/Input/IA_CameraLook.IA_CameraLook"))
  (bind (_x _y) (`KismetMathLibrary.BreakVector2D` ActionValue))
  (:`Triggered`
    (`self.CameraLookX` _x)
    (`self.CameraLookY` _y)))

(event `EnhancedInput|/Game/Input/IA_Reset`
  (params (ActionValue :type Boolean) (ElapsedSeconds :type "Float (double-precision)") (TriggeredSeconds :type "Float (double-precision)") (InputAction :type "InputAction Object Reference" :default "/Game/Input/IA_Reset.IA_Reset"))
  (:`Triggered`
    (`self.ResetPosition`)))

(event `EnhancedInput|/Game/Input/IA_Handbrake`
  (params (ActionValue :type Boolean) (ElapsedSeconds :type "Float (double-precision)") (TriggeredSeconds :type "Float (double-precision)") (InputAction :type "InputAction Object Reference" :default "/Game/Input/IA_Handbrake.IA_Handbrake"))
  (:`Triggered`
    (`self.ApplyHandbrake`))
  (:`Completed`
    (set `self.bUseHandbrake` false)))

(fn `UserConstructionScript`)