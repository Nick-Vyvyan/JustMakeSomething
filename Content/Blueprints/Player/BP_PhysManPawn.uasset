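; BP_PhysManPawn is a player pawn that moves by applying physics forces to a Sphere component.
; Four Enhanced Input actions push it forward, back, right and left along the forward and right vectors of the WorldForwardArrow component, scaled by ForceMultiplier.
; Forces apply as acceleration changes, so thrust is independent of the sphere's mass.
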(event `EnhancedInput|/Game/Input/InputActions/IA_PushForward`
  (params (ActionValue :type Boolean) (ElapsedSeconds :type "Float (double-precision)") (TriggeredSeconds :type "Float (double-precision)") (InputAction :type "InputAction Object Reference" :default "/Game/Input/InputActions/IA_PushForward.IA_PushForward"))
  ;[0.4297 0 1] Forward Thrust
  (:`Triggered`
    (`PrimitiveComponent.AddForce` (`self.Sphere`) (* (`SceneComponent.GetForwardVector` (`self.WorldForwardArrow`)) (`self.ForceMultiplier`)) "None" true)))

(event `EnhancedInput|/Game/Input/InputActions/IA_PushBack`
  (params (ActionValue :type Boolean) (ElapsedSeconds :type "Float (double-precision)") (TriggeredSeconds :type "Float (double-precision)") (InputAction :type "InputAction Object Reference" :default "/Game/Input/InputActions/IA_PushBack.IA_PushBack"))
  ;[1 0.4453 0] Backward Thrust
  (:`Triggered`
    (`PrimitiveComponent.AddForce` (`self.Sphere`) (* (* (`SceneComponent.GetForwardVector` (`self.WorldForwardArrow`)) -1.0) (`self.ForceMultiplier`)) "None" true)))

(event `EnhancedInput|/Game/Input/InputActions/IA_PushRight`
  (params (ActionValue :type Boolean) (ElapsedSeconds :type "Float (double-precision)") (TriggeredSeconds :type "Float (double-precision)") (InputAction :type "InputAction Object Reference" :default "/Game/Input/InputActions/IA_PushRight.IA_PushRight"))
  ;[0.9922 1 0] Right Thrust
  (:`Triggered`
    (`PrimitiveComponent.AddForce` (`self.Sphere`) (* (`SceneComponent.GetRightVector` (`self.WorldForwardArrow`)) (`self.ForceMultiplier`)) "None" true)))

(event `EnhancedInput|/Game/Input/InputActions/IA_PushLeft`
  (params (ActionValue :type Boolean) (ElapsedSeconds :type "Float (double-precision)") (TriggeredSeconds :type "Float (double-precision)") (InputAction :type "InputAction Object Reference" :default "/Game/Input/InputActions/IA_PushLeft.IA_PushLeft"))
  ;[1 0 0.6797] Left Thrust
  (:`Triggered`
    (`PrimitiveComponent.AddForce` (`self.Sphere`) (* (* (`SceneComponent.GetRightVector` (`self.WorldForwardArrow`)) -1) (`self.ForceMultiplier`)) "None" true)))

(fn `UserConstructionScript`)