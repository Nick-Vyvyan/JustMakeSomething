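; Game mode for a roller ball game that builds and extends a line of platforms as the player progresses.
; On BeginPlay it spawns a platform just below each PlayerStart, chains several more after the last, and shows the platform count widget.
; Each PlatformPassed event increments the passed count and appends another platform.
; The current tail platform spawns its successor, which becomes the new tail.
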(event `self.ReceiveBeginPlay`
  (`self.MakeStarterPlatforms`)
  (bind _returnvalue (`|CreateWidget` "/Game/UI/WBP_PlatformCount.WBP_PlatformCount_C"))
  (`UserWidget.AddToViewport` _returnvalue 0))

(event `PlatformPassed`
  (`/Engine/EditorBlueprintResources/StandardMacros.IncrementInt` (`self.PlatformsPassed`)
    (:`  `
      (`self.AddPlatformToEnd`))))

(fn `AddPlatformToEnd`
  (bind _asbp_platform_base (cast `/Game/Blueprints/Platforms/BP_PlatformBase` (`self.LastPlatformInLine`)))
  (bind _newplatform (`/Game/Blueprints/Platforms/BP_PlatformBase.SpawnNextPlatform` _asbp_platform_base))
  (set `self.LastPlatformInLine` _newplatform))

(fn `MakeStarterPlatforms`
  (bind _outactors (`GameplayStatics.GetAllActorsOfClass` "/Script/Engine.PlayerStart"))
  (for _array_element _outactors
    (bind _returnvalue (`|SpawnActorFromClass` "/Game/Blueprints/Platforms/BP_PlatformBase.BP_PlatformBase_C" (`KismetMathLibrary.Conv_VectorToTransform` (- (`self.K2_GetActorLocation` _array_element) (50.0 0.0 200.0))) "Undefined" "MultiplyWithRoot" null null))
    (set `self.LastPlatformInLine` _returnvalue))
  (for _ (range 6)
    (`self.AddPlatformToEnd`)))

(fn `UserConstructionScript`)