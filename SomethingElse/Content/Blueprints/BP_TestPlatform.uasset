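; BP_TestPlatform is a self-chaining platform actor that keeps spawning the next segment as the player advances.
; When a PlayerPawn overlaps EndTrigger, it spawns a new BP_TestPlatform at the NextSpawnLocation component's world position and then destroys itself.
; A separate KillTrigger detects the PlayerPawn falling and only prints a death message, with no further death handling.
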(event `self.EndTrigger.OnComponentBeginOverlap`
  (params (OverlappedComponent :type "PrimitiveComponent Object Reference") (OtherActor :type "Actor Object Reference") (OtherComp :type "PrimitiveComponent Object Reference") (OtherBodyIndex :type Integer) (bFromSweep :type Boolean) (SweepResult :type "HitResult Structure (by ref)"))
  (bind _asplayer_pawn (cast `PlayerPawn` OtherActor))
  (`/Engine/EditorBlueprintResources/StandardMacros.IsValid` _asplayer_pawn
    (:`Is Valid`
      (`|SpawnActorFromClass` "BP_TestPlatform_C" (`KismetMathLibrary.Conv_VectorToTransform` (`SceneComponent.K2_GetComponentLocation` (`self.NextSpawnLocation`))) "Undefined" "MultiplyWithRoot" null null)
      (`self.K2_DestroyActor`))))

(event `self.KillTrigger.OnComponentBeginOverlap`
  (params (OverlappedComponent :type "PrimitiveComponent Object Reference") (OtherActor :type "Actor Object Reference") (OtherComp :type "PrimitiveComponent Object Reference") (OtherBodyIndex :type Integer) (bFromSweep :type Boolean) (SweepResult :type "HitResult Structure (by ref)"))
  (bind _asplayer_pawn (cast `PlayerPawn` OtherActor))
  (`/Engine/EditorBlueprintResources/StandardMacros.IsValid` _asplayer_pawn
    (:`Is Valid`
      (`KismetSystemLibrary.PrintString` "Player Fell and Died" true true (struct :`G` 0.66 :`B` 1.0 :`A` 1.0) 5.0))))

(fn `UserConstructionScript`)