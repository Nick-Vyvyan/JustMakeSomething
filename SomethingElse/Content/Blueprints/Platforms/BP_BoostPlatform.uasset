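; BP_BoostPlatform is a platform that speeds up the player when they touch one of its three boost trigger volumes.
; Each trigger's overlap event casts the other actor to PlayerPawn and applies an impulse to its mesh along the pawn's ForwardArrow, scaled by BoostAmount.
; The impulse is a velocity change, so it ignores mass, and the identical logic is repeated per trigger with a debug print.
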(event `self.BoostTrigger.OnComponentBeginOverlap`
  (params (OverlappedComponent :type "PrimitiveComponent Object Reference") (OtherActor :type "Actor Object Reference") (OtherComp :type "PrimitiveComponent Object Reference") (OtherBodyIndex :type Integer) (bFromSweep :type Boolean) (SweepResult :type "HitResult Structure (by ref)"))
  (bind _asplayer_pawn (cast `PlayerPawn` OtherActor))
  (`/Engine/EditorBlueprintResources/StandardMacros.IsValid` _asplayer_pawn
    (:`Is Valid`
      (`PrimitiveComponent.AddImpulse` (`PlayerPawn.Mesh` _asplayer_pawn) (* (`SceneComponent.GetForwardVector` (`PlayerPawn.ForwardArrow` _asplayer_pawn)) (`self.BoostAmount`)) "None" true)
      (`KismetSystemLibrary.PrintString` "Boost!"))))

(event `self.BoostTrigger1.OnComponentBeginOverlap`
  (params (OverlappedComponent :type "PrimitiveComponent Object Reference") (OtherActor :type "Actor Object Reference") (OtherComp :type "PrimitiveComponent Object Reference") (OtherBodyIndex :type Integer) (bFromSweep :type Boolean) (SweepResult :type "HitResult Structure (by ref)"))
  (bind _asplayer_pawn (cast `PlayerPawn` OtherActor))
  (`/Engine/EditorBlueprintResources/StandardMacros.IsValid` _asplayer_pawn
    (:`Is Valid`
      (`PrimitiveComponent.AddImpulse` (`PlayerPawn.Mesh` _asplayer_pawn) (* (`SceneComponent.GetForwardVector` (`PlayerPawn.ForwardArrow` _asplayer_pawn)) (`self.BoostAmount`)) "None" true)
      (`KismetSystemLibrary.PrintString` "Boost!"))))

(event `self.BoostTrigger2.OnComponentBeginOverlap`
  (params (OverlappedComponent :type "PrimitiveComponent Object Reference") (OtherActor :type "Actor Object Reference") (OtherComp :type "PrimitiveComponent Object Reference") (OtherBodyIndex :type Integer) (bFromSweep :type Boolean) (SweepResult :type "HitResult Structure (by ref)"))
  (bind _asplayer_pawn (cast `PlayerPawn` OtherActor))
  (`/Engine/EditorBlueprintResources/StandardMacros.IsValid` _asplayer_pawn
    (:`Is Valid`
      (`PrimitiveComponent.AddImpulse` (`PlayerPawn.Mesh` _asplayer_pawn) (* (`SceneComponent.GetForwardVector` (`PlayerPawn.ForwardArrow` _asplayer_pawn)) (`self.BoostAmount`)) "None" true)
      (`KismetSystemLibrary.PrintString` "Boost!"))))

(fn `UserConstructionScript`
  (`parent.UserConstructionScript`))