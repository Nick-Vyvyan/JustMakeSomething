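; BP_PlatformBase is a platform actor for a roller-ball game that can spawn a successor and removes itself once passed.
; On BeginPlay it copies the platform class list from RollerBallGameMode, which SpawnNextPlatform uses to spawn a random platform at NextSpawnLocation.
; When the player pawn overlaps EndTrigger, it notifies BP_RollerBallGameMode, then destroys itself after a short delay.
; KillTrigger only prints a death message; SpawnNextPlatform is not called within this Blueprint.
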(event `self.ReceiveBeginPlay`
  (bind _asroller_ball_game_mode (cast `RollerBallGameMode` (`GameplayStatics.GetGameMode`)))
  (`/Engine/EditorBlueprintResources/StandardMacros.IsValid` _asroller_ball_game_mode
    (:`Is Valid`
      (set `self.Platform Class Array` (`RollerBallGameMode.PlatformClassArray` _asroller_ball_game_mode)))))

(event `self.EndTrigger.OnComponentBeginOverlap`
  (params (OverlappedComponent :type "PrimitiveComponent Object Reference") (OtherActor :type "Actor Object Reference") (OtherComp :type "PrimitiveComponent Object Reference") (OtherBodyIndex :type Integer) (bFromSweep :type Boolean) (SweepResult :type "HitResult Structure (by ref)"))
  (bind _asplayer_pawn (cast `PlayerPawn` OtherActor))
  (`/Engine/EditorBlueprintResources/StandardMacros.IsValid` _asplayer_pawn
    (:`Is Valid`
      (bind _asbp_roller_ball_game_mode (cast `/Game/Blueprints/BP_RollerBallGameMode` (`GameplayStatics.GetGameMode`)))
      (`/Game/Blueprints/BP_RollerBallGameMode.PlatformPassed` _asbp_roller_ball_game_mode)
      (`KismetSystemLibrary.Delay` 2.0)
      (`self.K2_DestroyActor`))))

(event `self.KillTrigger.OnComponentBeginOverlap`
  (params (OverlappedComponent :type "PrimitiveComponent Object Reference") (OtherActor :type "Actor Object Reference") (OtherComp :type "PrimitiveComponent Object Reference") (OtherBodyIndex :type Integer) (bFromSweep :type Boolean) (SweepResult :type "HitResult Structure (by ref)"))
  (bind _asplayer_pawn (cast `PlayerPawn` OtherActor))
  (`/Engine/EditorBlueprintResources/StandardMacros.IsValid` _asplayer_pawn
    (:`Is Valid`
      (`KismetSystemLibrary.PrintString` "Player Fell and Died" true true (struct :`G` 0.66 :`B` 1.0 :`A` 1.0) 5.0))))

(fn `SpawnNextPlatform`
  (returns (NewPlatform :type "PlatformBase Object Reference"))
  (bind _returnvalue (`|SpawnActorFromClass` (`KismetArrayLibrary.Array_Random` (`self.Platform Class Array`)) (`KismetMathLibrary.Conv_VectorToTransform` (`SceneComponent.K2_GetComponentLocation` (`self.NextSpawnLocation`))) "Undefined" "MultiplyWithRoot" null null))
  (return _returnvalue))

(fn `UserConstructionScript`)