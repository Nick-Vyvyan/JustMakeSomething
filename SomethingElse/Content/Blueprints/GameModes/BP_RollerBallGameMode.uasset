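; Game mode for a roller-ball endless platform game that builds the track and tracks the high score.
; BeginPlay loads any saved high score, spawns a platform under the PlayerStart, chains more after it, and shows platform-count and high-score widgets.
; Each PlatformPassed event increments the count, has the last platform spawn its successor, and writes a matched or beaten high score to the save slot.
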(event `self.ReceiveBeginPlay`
  (bind _returnvalue (`GameplayStatics.DoesSaveGameExist` (`self.Slot Name`)))
  (if _returnvalue
    (bind _returnvalue_2 (`GameplayStatics.LoadGameFromSlot` (`self.Slot Name`)))
    (bind _output_get (set `self.SaveSubclass` _returnvalue_2))
    (bind _asbp_save_high_score (cast `/Game/Blueprints/BP_SaveHighScore` _output_get))
    (set `self.HighScore` (`/Game/Blueprints/BP_SaveHighScore.HighScore` _asbp_save_high_score)))
  (`self.MakeStarterPlatforms`)
  (bind _returnvalue_3 (`|CreateWidget` "/Game/UI/WBP_PlatformCount.WBP_PlatformCount_C"))
  (`UserWidget.AddToViewport` _returnvalue_3 0)
  (bind _returnvalue_4 (`|CreateWidget` "/Game/UI/WBP_HighScore.WBP_HighScore_C"))
  (`UserWidget.AddToViewport` _returnvalue_4 0))

(event `PlatformPassed`
  (bind _platformspassed (`self.PlatformsPassed`))
  (bind _slot_name (`self.Slot Name`))
  (bind _savesubclass (`self.SaveSubclass`))
  (`/Engine/EditorBlueprintResources/StandardMacros.IncrementInt` (`self.PlatformsPassed`)
    (:`  `
      (`self.AddPlatformToEnd`)
      (if (>= _platformspassed (`self.HighScore`))
        (set `self.HighScore` _platformspassed)
        (bind _returnvalue (`GameplayStatics.DoesSaveGameExist` (`self.Slot Name`)))
        (if _returnvalue
          (bind _returnvalue_2 (`GameplayStatics.LoadGameFromSlot` (`self.Slot Name`)))
          (bind _output_get (set `self.SaveSubclass` _returnvalue_2))
          (bind _asbp_save_high_score (cast `/Game/Blueprints/BP_SaveHighScore` _output_get))
          (set `/Game/Blueprints/BP_SaveHighScore.HighScore` (`self.HighScore`) _asbp_save_high_score)
          (`GameplayStatics.SaveGameToSlot` _savesubclass _slot_name)
          (else
            (bind _returnvalue_3 (`GameplayStatics.CreateSaveGameObject` "/Game/Blueprints/BP_SaveHighScore.BP_SaveHighScore_C"))
            (bind _output_get_2 (set `self.SaveSubclass` _returnvalue_3))
            (bind _asbp_save_high_score_2 (cast `/Game/Blueprints/BP_SaveHighScore` _output_get_2))
            (set `/Game/Blueprints/BP_SaveHighScore.HighScore` (`self.HighScore`) _asbp_save_high_score_2)
            (`GameplayStatics.SaveGameToSlot` _savesubclass _slot_name)))))))

(fn `AddPlatformToEnd`
  (bind _asbp_platform_base (cast `/Game/Blueprints/Platforms/BP_PlatformBase` (`self.LastPlatformInLine`)))
  (bind _newplatform (`/Game/Blueprints/Platforms/BP_PlatformBase.SpawnNextPlatform` _asbp_platform_base))
  (set `self.LastPlatformInLine` _newplatform))

(fn `MakeStarterPlatforms`
  (bind _outactors (`GameplayStatics.GetAllActorsOfClass` "/Script/Engine.PlayerStart"))
  (for _array_element _outactors
    (bind _returnvalue (`|SpawnActorFromClass` "/Game/Blueprints/Platforms/BP_PlatformBase.BP_PlatformBase_C" (`KismetMathLibrary.Conv_VectorToTransform` (- (`self.K2_GetActorLocation` _array_element) (50.0 0.0 200.0))) "Undefined" "MultiplyWithRoot" null null))
    (set `self.LastPlatformInLine` _returnvalue))
  (for _ (range 6)
    (`self.AddPlatformToEnd`)))

(fn `UserConstructionScript`)